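; BP_SkateCharacter is a skating character Blueprint that feeds movement speed to its mesh's animation instance.
; It pushes max speed to the anim instance on BeginPlay and the current velocity magnitude every Tick.
; Tick also shifts the mesh's relative Y, easing it toward a negative offset while moving and snapping it back to zero when stopped.
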(event EventBeginPlay
  (|CallParentFunction)
  (Class|BPIAnimBP|PushMaxSpeed(Message) (Components|SkeletalMesh|GetAnimInstance (Variables|Character|GetMesh)) (Class|MovementComponent|GetMaxSpeed (Variables|Character|GetCharacterMovement))))

(event Collision|EventActorBeginOverlap
  (params (OtherActor :type Actor%20Object%20Reference)))

(event EventTick
  (params (DeltaSeconds :type Float%20%28single-precision%29))
  (bind _charactermovement (Variables|Character|GetCharacterMovement))
  (bind _mesh (Variables|Character|GetMesh))
  (bind _velocity (Variables|/Script/Engine.MovementComponent|GetVelocity _charactermovement))
  (bind _relativelocation (Variables|/Script/Engine.SceneComponent|GetRelativeLocation _mesh))
  (bind _returnvalue (Math|Vector|VectorLength _velocity))
  (|CallParentFunction DeltaSeconds)
  (Class|BPIAnimBP|PushSpeed(Message) (Components|SkeletalMesh|GetAnimInstance (Variables|Character|GetMesh)) _returnvalue)
  (Transformation|SetRelativeLocation (Variables|Character|GetMesh) (Math|Vector|MakeVector (.x _relativelocation) (Math|Float|SelectFloat (Math|Interpolation|FInterpTo (.y _relativelocation) -2e+01 DeltaSeconds 1.0) 0.0 (> _returnvalue 0.0)) (.z _relativelocation)) false false))

(fn ConstructionScript)